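; BP_BotCharacter is a robot character that is assigned an owner and can be talked to through interaction.
; On BeginPlay it binds to its OnInitialized event, then hands the received owner to its AIC_Bot controller, printing debug text for success or failure.
; Interacting through InteractableCmp calls ServerExecuteTalkCommand with a hard-coded "Talk" command and prompt message.
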(event `self.ReceiveBeginPlay`
  (add `self.OnInitialized` (delegate `OnInitialized_Event`)))

(event `OnInitialized_Event` :!signature `self.OnInitialized`
  (params (BotOwner :type "Actor Object Reference"))
  (`self.OwnerChange` BotOwner))

(event `self.InteractableCmp.OnInteract`
  (params (Interactor :type "Actor Object Reference"))
  (`self.ServerExecuteTalkCommand` "Talk" "What could we do around here"))

(fn `OwnerChange`
  (params (Owner :type "Actor Object Reference"))
  (bind _returnvalue (`AIBlueprintHelperLibrary.GetAIController` self))
  (`/Engine/EditorBlueprintResources/StandardMacros.IsValid` Owner
    (:`Is Valid`
      (bind _asaic_bot (cast `/Game/SNP/Robot/AIC_Bot` _returnvalue)
        (:`then`
          (`/Game/SNP/Robot/AIC_Bot.SetBotOwner` _asaic_bot Owner)
          (`KismetSystemLibrary.PrintString` "Bot owner set correctly"))
        (:`CastFailed`
          (`KismetSystemLibrary.PrintString` (`KismetSystemLibrary.GetDisplayName` _returnvalue)))))
    (:`Is Not Valid`
      (`KismetSystemLibrary.PrintString` "Owner is null"))))

(fn `UserConstructionScript`)